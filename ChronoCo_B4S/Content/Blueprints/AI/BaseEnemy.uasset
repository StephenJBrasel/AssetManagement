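; BaseEnemy is an AI enemy that acts as a suicide attacker against the player.
; When PawnSensing sees a pawn, it fetches the player's ThirdPersonCharacter and uses AI MoveTo to chase it.
; On reaching it, the enemy destroys itself with an explosion effect and sound, then passes Damage to the player's ChangeHealth.
; Mesh impulse and rifle socket attachment nodes are present but disconnected.
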(event OnSeePawn(PawnSensing)
  (params (Pawn :type Pawn%20Object%20Reference))
  (bind _returnvalue (Transformation|GetActorLocation))
  (bind _asthird_person_character (Utilities|Casting|CastToThirdPersonCharacter (Game|GetPlayerCharacter 0)))
  (AI|AIMoveTo self "0, 0, 0" _asthird_person_character 1.0 false
    (:OnSuccess
      (Actor|DestroyActor)
      (Effects|SpawnEmitteratLocation "/Game/StarterContent/Particles/P_Explosion.P_Explosion" _returnvalue)
      (Audio|PlaySoundatLocation "/Game/StarterContent/Audio/Explosion01.Explosion01" _returnvalue "0, 0, 0" 1.0 1.0 0.0 0 0 0)
      (Default|ChangeHealth _asthird_person_character (Variables|Default|GetDamage) true))))

(fn ConstructionScript)