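; AI spawner actor that spawns pawns with a behavior tree at its own transform after a start delay.
; CreatePawn picks each class as singular, random or cycled from AIVarieties.
; Tick spawns more up to a count limit, but TimeSinceLast resets to zero, so the interval compares against total real time rather than spacing spawns.
; SlowTime temporarily lowers or changes the actor's CustomTimeDilation, scaling its restore delay by that dilation.
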(event Custom|SlowTime
  (params (TimeDilation :type Float%20%28single-precision%29) (TimeDuration :type Float%20%28single-precision%29))
  ;[1 1 1] SetTimeSlowComponents
  (Variables|TimeSlow|SetSlowed true)
  (Variables|TimeSlow|SetDilation TimeDilation)
  (Variables|TimeSlow|SetDuration TimeDuration))

(event Collision|EventActorBeginOverlap
  (params (OtherActor :type Actor%20Object%20Reference)))

(event EventTick
  (params (DeltaSeconds :type Float%20%28single-precision%29))
  (bind _maxspawncount (Variables|Default|GetMaxSpawnCount))
  (Utilities|FlowControl|Sequence
    (:then_0
      ;[1 1 1] Spawn AI
      (if (Math|Boolean|ANDBoolean (and (<= (Variables|Default|GetNumSpawn) _maxspawncount) (!= _maxspawncount 0)) (>= (Variables|Default|GetSecondsBetweenSpawn) 0.0) (Variables|Default|GetIsSpawning) (>= (- (Utilities|Time|GetRealTimeSeconds) (Variables|Default|GetTimeSinceLast)) (Variables|Default|GetSecondsBetweenSpawn)))
        (bind _spawnpawn (CallFunction|CreatePawn (Variables|Default|GetSpawningMethod)))
        (CallFunction|SpawnAI _spawnpawn (Variables|Default|GetAIBehaviorTree))
        (Variables|Default|SetTimeSinceLast 0.0)
        (Math|Integer|IncrementInt (Variables|Default|GetNumSpawn))))
    (:then_1
      ;[1 1 1] SlowTimeFunction
      (if (Variables|TimeSlow|GetSlowed)
        (bind _output_get (Variables|Default|SetCustomTimeDilation (Variables|TimeSlow|GetDilation)))
        (Utilities|FlowControl|Delay (* (Variables|TimeSlow|GetDuration) _output_get))
        (Variables|Default|SetCustomTimeDilation 1.0)
        (Variables|TimeSlow|SetSlowed false)))))

(event EventBeginPlay
  (bind _returnvalue (Utilities|Time|GetRealTimeSeconds))
  ;[1 1 1] Wait, then spawn
  (Development|PrintString (Utilities|String|ToString(Float) _returnvalue))
  (Utilities|FlowControl|Delay (Variables|Default|GetSecondsBeforeSpawningStarts))
  (Development|PrintString (Utilities|String|ToString(Float) _returnvalue))
  (Variables|Default|SetIsSpawning true)
  (bind _spawnpawn (CallFunction|CreatePawn (Variables|Default|GetSpawningMethod)))
  (CallFunction|SpawnAI _spawnpawn (Variables|Default|GetAIBehaviorTree))
  (Variables|Default|SetTimeSinceLast 0.0))

(fn ConstructionScript)

(fn SpawnAI
  (params (PawnClass :type Pawn%20Class%20Reference) (BehaviorTree :type Behavior%20Tree%20Object%20Reference))
  (bind _returnvalue (Transformation|GetActorTransform))
  (bind (_location _rotation) (Math|Transform|BreakTransform _returnvalue))
  (bind _returnvalue_2 (AI|SpawnAIFromClass PawnClass BehaviorTree _location _rotation false))
  (return _returnvalue_2))

(fn CreatePawn
  (params (SpawningMethod :type SpawnMethod%20Enum :default "NewEnumerator1"))
  (switch Utilities|FlowControl|Switch|SwitchonSpawnMethod SpawningMethod
    (:NewEnumerator1
      (LocalVariables|SetSpawnClassReturn (Variables|Default|GetSpawningAI)))
    (:NewEnumerator2
      (LocalVariables|SetSpawnClassReturn (Utilities|Array|Get(acopy) (Variables|Default|GetAIVarieties) (Math|Random|RandomInteger (Utilities|Array|Length (Variables|Default|GetAIVarieties))))))
    (:NewEnumerator3
      ;[1 1 1] Cycle
      (bind _result (Math|Integer|IncrementInt (Variables|Default|GetCurrentAISpawnClassIndex))
        (:%20%20
          (LocalVariables|SetSpawnClassReturn (Utilities|Array|Get(acopy) (Variables|Default|GetAIVarieties) (Math|Integer|%(Integer) _result (Utilities|Array|Length (Variables|Default|GetAIVarieties)))))))))
  (return (LocalVariables|GetSpawnClassReturn)))