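; TimedSpawner is an actor that repeatedly spawns SpawnClass at its own transform.
; Tick feeds a Delay of SecondsBetweenSpawns, which paces the spawns because calls made while it is pending are ignored.
; SpawnCount increments while MaxSpawnCount is nonzero and not exceeded, but SpawnActor runs outside that check, so the limit does not stop spawning.
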(event EventBeginPlay)

(event Collision|EventActorBeginOverlap
  (params (OtherActor :type Actor%20Object%20Reference)))

(event EventTick
  (params (DeltaSeconds :type Float%20%28single-precision%29))
  (Utilities|FlowControl|Delay (Variables|Default|GetSecondsBetweenSpawns))
  (if (and (!= (Variables|Default|GetMaxSpawnCount) 0) (<= (Variables|Default|GetSpawnCount) (Variables|Default|GetMaxSpawnCount)))
    (Math|Integer|IncrementInt (Variables|Default|GetSpawnCount)
      (:%20%20
        _)))
  (Game|SpawnActorfromClass (Variables|Default|GetSpawnClass) (Transformation|GetActorTransform) "Undefined" 0 0))

(fn ConstructionScript)