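; Blue bouncy ball test actor that destroys itself after its LifeTime and can be individually slowed in time.
; The SlowTime event stores a dilation and duration and sets a Slowed flag.
; While flagged, Tick applies the CustomTimeDilation, waits for the duration multiplied by that dilation, then restores normal speed and clears the flag.
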(event Custom|SlowTime
  (params (TimeDilation :type Float%20%28single-precision%29) (TimeDuration :type Float%20%28single-precision%29))
  ;[1 1 1] SetTimeSlowComponents
  (Variables|Default|SetSlowed true)
  (Variables|Default|SetDilation TimeDilation)
  (Variables|Default|SetDuration TimeDuration))

(event Collision|EventActorBeginOverlap
  (params (OtherActor :type Actor%20Object%20Reference)))

(event EventTick
  (params (DeltaSeconds :type Float%20%28single-precision%29))
  ;[1 1 1] SlowTimeFunction
  (if (Variables|Default|GetSlowed)
    (bind _output_get (Variables|Default|SetCustomTimeDilation (Variables|Default|GetDilation)))
    (Utilities|FlowControl|Delay (* (Variables|Default|GetDuration) _output_get))
    (Variables|Default|SetCustomTimeDilation 1.0)
    (Variables|Default|SetSlowed false)))

(event EventBeginPlay
  (Utilities|FlowControl|Delay (Variables|Default|GetLifeTime))
  (Actor|DestroyActor))

(fn ConstructionScript)