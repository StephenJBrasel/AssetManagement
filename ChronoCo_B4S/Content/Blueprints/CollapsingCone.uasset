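; CollapsingCone is an actor that starts a collapse after the player character has overlapped it for a set delay.
; Tick polls the overlap, counts the delay down, then calls StartCollapse on ComponentCollapse every frame while contact lasts.
; Without overlap, the delay recovers at a scaled rate up to its BeginPlay value, and PauseCollapse fires once after contact ends.
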(event EventBeginPlay
  (Variables|Default|SetStartTime (Variables|Default|GetDelayBeforeStartCollapse)))

(event EventTick
  (params (DeltaSeconds :type Float%20%28single-precision%29))
  (bind _returnvalue (Game|GetPlayerCharacter 0))
  (bind _componentcollapse (Variables|Default|GetComponentCollapse))
  (bind _componentcollapse_2 (Variables|Default|GetComponentCollapse))
  ;[1 1 1] Detect Collapse
  (if (Collision|IsOverlappingActor _returnvalue :!class /Script/Engine.Actor)
    ;[1 1 1] Begin Collapse
    (Variables|Default|SetBeganCollapse true)
    (if (Variables|Default|GetBeganCollapse)
      (Utilities|Casting|CastToThirdPersonCharacter _returnvalue)
      (if (<= (Variables|Default|GetDelayBeforeStartCollapse) 0.0)
        (Utilities|IsValid _componentcollapse
          (:Is%20Valid
            (Default|StartCollapse _componentcollapse _returnvalue)
            (Variables|Default|SetPauseCollapse false)))
        (else
          (Variables|Default|SetDelayBeforeStartCollapse (- (Variables|Default|GetDelayBeforeStartCollapse) DeltaSeconds)))))
    (else
      ;[1 1 1] PauseCollapse
      (bind _output_get (Variables|Default|SetPauseCollapse true))
      (if _output_get
        (Variables|Default|SetDelayBeforeStartCollapse (Math|Float|Clamp(Float) (+ (Variables|Default|GetDelayBeforeStartCollapse) (* DeltaSeconds (Variables|Default|GetCollapseRecoveryFactor))) 0.0 (Variables|Default|GetStartTime)))
        (if (Variables|Default|GetBeganCollapse)
          (Utilities|Casting|CastToThirdPersonCharacter _returnvalue)
          (Utilities|IsValid _componentcollapse_2
            (:Is%20Valid
              (Default|PauseCollapse _componentcollapse_2 _returnvalue)
              (Variables|Default|SetBeganCollapse false))))))))

(fn ConstructionScript)