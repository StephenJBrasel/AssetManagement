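; Moving platform actor that oscillates around the location it records at BeginPlay.
; Each Tick sums sine offsets along its right and forward vectors and a cosine offset along its up vector, each with its own speed and magnitude, driven by real time.
; Logic to multiply or divide the speeds for an overlapping ThirdPersonCharacter exists but is disconnected, so both overlap events do nothing.
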(event EventBeginPlay
  (Variables|Default|SetStartLocation (Transformation|GetActorLocation)))

(event Collision|EventActorBeginOverlap
  (params (OtherActor :type Actor%20Object%20Reference))
  ;[1 1 1] Speed Up
)

(event EventTick
  (params (DeltaSeconds :type Float%20%28single-precision%29))
  (bind _returnvalue (Utilities|Time|GetRealTimeSeconds))
  (Transformation|SetActorLocationAndRotation (+ (Variables|Default|GetStartLocation) (* (Transformation|GetActorRightVector) (* (Math|Trig|Sin(Radians) (* _returnvalue (Variables|Default|GetXSpeed))) (Variables|Default|GetXMagnitude))) (* (Transformation|GetActorUpVector) (* (Math|Trig|Cos(Radians) (* _returnvalue (Variables|Default|GetYSpeed))) (Variables|Default|GetYMagntiude))) (* (Transformation|GetActorForwardVector) (* (Math|Trig|Sin(Radians) (* _returnvalue (Variables|Default|GetZSpeed))) (Variables|Default|GetZMagnitude)))) (Transformation|GetActorRotation)))

(event Collision|EventActorEndOverlap
  (params (OtherActor :type Actor%20Object%20Reference))
  ;[1 1 1] Slow Down
)

(fn ConstructionScript)