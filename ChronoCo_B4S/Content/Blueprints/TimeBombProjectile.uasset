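; A time bomb projectile that triggers a localized time slow where it hits and expires after a set lifetime.
; On hit it pushes physics-simulating components with a velocity-scaled impulse, shows an effect mesh, then hides the collision component and its children after a short delay.
; It delegates the slow to the player's ThirdPersonCharacter, passing position, radius, dilation and duration, then destroys itself.
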(event EventBeginPlay
  (Utilities|FlowControl|Delay (Variables|Default|GetLifeTime))
  (Actor|DestroyActor))

(event Collision|EventActorBeginOverlap
  (params (OtherActor :type Actor%20Object%20Reference)))

(event EventTick
  (params (DeltaSeconds :type Float%20%28single-precision%29)))

(event Collision|EventHit
  (params (MyComp :type Primitive%20Component%20Object%20Reference) (Other :type Actor%20Object%20Reference) (OtherComp :type Primitive%20Component%20Object%20Reference) (bSelfMoved :type Boolean) (HitLocation :type Vector :default "0, 0, 0") (HitNormal :type Vector :default "0, 0, 0") (NormalImpulse :type Vector :default "0, 0, 0") (Hit :type Hit%20Result%20Structure%20%28by%20ref%29))
  (bind _returnvalue (Transformation|GetActorLocation))
  ;[1 1 1] Slows Time, Adds physics impulse to any physics object we hit
  (bind _asthird_person_character (Utilities|Casting|CastToThirdPersonCharacter (Game|GetPlayerCharacter 0)))
  (if (Physics|IsSimulatingPhysics OtherComp "None")
    (Physics|AddImpulseatLocation OtherComp (* (Transformation|GetVelocity) 1e+02) _returnvalue "None"))
  (Rendering|SetVisibility (Variables|Default|GetTimeBombEffectMesh) true false)
  (Utilities|FlowControl|Delay 0.2)
  (Rendering|SetVisibility (Variables|Default|GetCollision%20Component) false true)
  (Default|EventSlowTime _asthird_person_character _returnvalue (Variables|Default|GetP_TimeBombRadius) (Variables|Default|GetP_TimeDilation) (Variables|Default|GetP_TimeSlowDuration))
  (Actor|DestroyActor) ; Then destroy this projectile
)

(fn ConstructionScript)