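; Actor component that turns its owner into a floating, collapsible platform, bobbing on sine/cosine offsets from a randomised start time.
; StartCollapse, given a ThirdPersonCharacter, halts motion, spawns one-time warning effects and runs a countdown.
; PauseCollapse resumes motion and keeps the remaining time.
; At zero, the mesh drops under physics with an explosion effect and sound, then the owner is destroyed after an optional linger.
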(event Custom|DestroyAfterCollapse
  (bind _collapsingaudioref (Variables|Default|GetCollapsingAudioRef))
  (bind _lingertimebeforedestroyed (Variables|Default|GetLingerTimeBeforeDestroyed))
  (bind _collapsingparticlesref (Variables|Default|GetCollapsingParticlesRef))
  ;[1 1 1] Destroy After Collapse
  (if (== _lingertimebeforedestroyed 0.0)
    _
    (else
      (Utilities|FlowControl|Delay _lingertimebeforedestroyed)))
  (Actor|DestroyActor (Components|GetOwner))
  (Utilities|IsValid _collapsingparticlesref
    (:Is%20Valid
      (Components|DestroyComponent _collapsingparticlesref))
    (:Is%20Not%20Valid
      _))
  (Utilities|IsValid _collapsingaudioref
    (:Is%20Valid
      (Components|DestroyComponent _collapsingaudioref))
    (:Is%20Not%20Valid
      _))
  (Components|DestroyComponent))

(event EventBeginPlay
  ;[1 1 1] Initialize
  (Variables|Default|SetStartLocation (Transformation|GetActorLocation (Components|GetOwner)))
  (if (== 0.0 (Variables|Default|GetCurrentTime))
    (Variables|Default|SetCurrentTime (Math|Random|RandomFloat))))

(event EventTick
  (params (DeltaSeconds :type Float%20%28single-precision%29))
  (bind _returnvalue (Components|GetOwner))
  (bind _returnvalue_2 (Components|GetOwner))
  (bind _collapsingparticlesref (Variables|Default|GetCollapsingParticlesRef))
  (bind _collapsingaudioref (Variables|Default|GetCollapsingAudioRef))
  (bind _meshclassoffallingactor (Variables|Components|GetMeshClassOfFallingActor))
  (bind _returnvalue_3 (Transformation|GetActorLocation _returnvalue_2))
  (bind _returnvalue_4 (Actor|GetComponentbyClass _returnvalue_2 _meshclassoffallingactor))
  (if (or (Variables|Default|GetCollapsing) (Variables|Default|GetCollapsed))
    (if (<= (Variables|Default|GetTimeBeforeCollapsed) 0.0)
      (if (not (Variables|Default|GetCollapsed))
        (Variables|Default|SetCollapsed true)
        ;[1 1 1] Collapsed
        (Utilities|IsValid _collapsingparticlesref
          (:Is%20Valid
            (Rendering|SetVisibility _collapsingparticlesref false false)
            (Collision|SetCollisionEnabled _collapsingparticlesref "NoCollision")
            (Components|DestroyComponent _collapsingparticlesref))
          (:Is%20Not%20Valid
            _))
        (Utilities|IsValid _collapsingaudioref
          (:Is%20Valid
            (Audio|Components|Audio|Stop _collapsingaudioref)
            (Components|DestroyComponent _collapsingaudioref))
          (:Is%20Not%20Valid
            _))
        (Physics|SetSimulatePhysics _returnvalue_4 true)
        (Physics|SetEnableGravity _returnvalue_4 true)
        (Effects|SpawnEmitteratLocation "/Game/StarterContent/Particles/P_Explosion.P_Explosion" _returnvalue_3)
        (Audio|PlaySoundatLocation "/Game/StarterContent/Audio/Explosion01.Explosion01" _returnvalue_3 "0, 0, 0" 1.0 1.0 0.0 0 0 (Components|GetOwner))
        (CallFunction|DestroyAfterCollapse))
      (else
        (Variables|Default|SetTimeBeforeCollapsed (- (Variables|Default|GetTimeBeforeCollapsed) DeltaSeconds))))
    (else
      ;[1 1 1] Moving Area/Moving Platform
      (Variables|Default|SetCurrentTime (+ (Variables|Default|GetCurrentTime) DeltaSeconds))
      (Transformation|SetActorLocationAndRotation _returnvalue (+ (Variables|Default|GetStartLocation) (* (Transformation|GetActorRightVector _returnvalue) (* (Math|Trig|Sin(Radians) (* (Variables|Default|GetCurrentTime) (Variables|Movement|GetXSpeed))) (Variables|Movement|GetXMagnitude))) (* (Transformation|GetActorUpVector _returnvalue) (* (Math|Trig|Cos(Radians) (* (Variables|Default|GetCurrentTime) (Variables|Movement|GetYSpeed))) (Variables|Movement|GetYMagntiude))) (* (Transformation|GetActorForwardVector _returnvalue) (* (Math|Trig|Sin(Radians) (* (Variables|Default|GetCurrentTime) (Variables|Movement|GetZSpeed))) (Variables|Movement|GetZMagnitude)))) (Transformation|GetActorRotation _returnvalue)))))

(fn StartCollapse
  (params (Object :type Object%20Object%20Reference))
  (bind _returnvalue (Components|GetOwner))
  (bind _collapsingsound (Variables|Components|GetCollapsingSound))
  (bind _collapsingparticles (Variables|Components|GetCollapsingParticles))
  (bind _returnvalue_2 (Transformation|GetActorLocation _returnvalue))
  ;[1 1 1] Collapsing
  (Utilities|Casting|CastToThirdPersonCharacter Object)
  (Utilities|IsValid _collapsingparticles
    (:Is%20Valid
      (Utilities|IsValid (Variables|Default|GetCollapsingParticlesRef)
        (:Is%20Valid
          _)
        (:Is%20Not%20Valid
          (if (Variables|Default|GethasSpawnedParticles)
            _
            (else
              (Variables|Default|SethasSpawnedParticles true)
              (bind _returnvalue_3 (Effects|SpawnEmitteratLocation _collapsingparticles _returnvalue_2 "0, 0, 0" "1.000000,1.000000,1.000000" false))
              (Variables|Default|SetCollapsingParticlesRef _returnvalue_3))))))
    (:Is%20Not%20Valid
      _))
  (Utilities|IsValid _collapsingsound
    (:Is%20Valid
      (Utilities|IsValid (Variables|Default|GetCollapsingAudioRef)
        (:Is%20Valid
          _)
        (:Is%20Not%20Valid
          (if (Variables|Default|GethasSpawnedAudio)
            _
            (else
              (Variables|Default|SethasSpawnedAudio true)
              (bind _returnvalue_4 (Audio|SpawnSoundatLocation _collapsingsound _returnvalue_2 "0, 0, 0" 1.0 1.0 0.0 0 0 false))
              (Variables|Default|SetCollapsingAudioRef _returnvalue_4))))))
    (:Is%20Not%20Valid
      _))
  (Variables|Default|SetCollapsing true))

(fn PauseCollapse
  (params (Other%20Actor :type Object%20Object%20Reference))
  (Utilities|Casting|CastToThirdPersonCharacter Other%20Actor)
  (Variables|Default|SetCollapsing false))